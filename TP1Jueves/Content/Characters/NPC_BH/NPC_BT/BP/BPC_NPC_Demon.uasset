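; BPC_NPC_Demon is a demon NPC character with a melee attack on the first-person player.
; AttackPlayer sphere-traces just ahead; a player hit plays an attack montage on the first demon found in the world, then damages the player, makes them jump and checks their life.
; AnyDamage only lowers VidaActual, while GetDamage lowers a separate MyLife and destroys the demon at zero.
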(event Custom|Attack%20Player
  (bind _returnvalue (Transformation|GetActorLocation))
  ;[1 1 1] Detección del player
  (bind (_outhit _returnvalue_2) (Collision|SphereTraceForObjects _returnvalue (+ _returnvalue (* (Math|Vector|GetForwardVector (Transformation|GetActorRotation)) 1e+02)) 7e+01 (Utilities|Array|MakeArray "ObjectTypeQuery3") false 0 "None"))
  (if _returnvalue_2
    (Utilities|Casting|CastToBP_FirstPersonCharacter (.HitActor (Collision|BreakHitResult _outhit)))
    (CallFunction|AnimationAttack)
    (CallFunction|PlayerDamage)))

(event Custom|AnimationAttack
  ;[1 1 1] correr animacion
  (bind _returnvalue (Actor|GetActorOfClass "BPC_NPC_Demon_C"))
  (Animation|Montage|PlayMontage (Variables|/Script/Engine.Character|GetMesh _returnvalue) "/Game/Characters/NPC_BH/NPC_BT/animations/AM_Demon.AM_Demon" 1.0 0.0 (Utilities|Array|Get(acopy) (Variables|Default|GetSecctions))))

(event Custom|PlayerDamage
  (bind _asbp_first_person_character (Utilities|Casting|CastToBP_FirstPersonCharacter (.HitActor (Collision|BreakHitResult (stale Custom|Attack%20Player _outhit)))))
  (bind _output_get (Variables|Default|SetBP_FirstPerson _asbp_first_person_character))
  (Variables|/Game/FirstPerson/Blueprints/BP_FirstPersonCharacter.BP_FirstPersonCharacter_C|SetVidaActual _output_get (- (Variables|/Game/FirstPerson/Blueprints/BP_FirstPersonCharacter.BP_FirstPersonCharacter_C|GetVidaActual _output_get) 1.0))
  (Character|Jump (Variables|Default|GetBP_FirstPerson))
  (Default|Checklife (Variables|Default|GetBP_FirstPerson)))

(event Game|Damage|EventAnyDamage
  (params (Damage :type Float%20%28single-precision%29) (DamageType :type Damage%20Type%20Object%20Reference) (InstigatedBy :type Controller%20Object%20Reference) (DamageCauser :type Actor%20Object%20Reference))
  ;[1 1 1] Resto vida enemigo
  (Variables|Default|SetVidaActual (- (Variables|Default|GetVidaActual) Damage)))

(fn ConstructionScript)

(fn GetDamage
  (params (damage :type Float%20%28double-precision%29))
  (bind _output_get (Variables|Default|SetMyLife (- (Variables|Default|GetMyLife) damage)))
  (if (<= _output_get 0.0)
    (Actor|DestroyActor)
    (else
      (Development|PrintText "recibi daño"))))