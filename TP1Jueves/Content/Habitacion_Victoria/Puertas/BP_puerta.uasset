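; Key-locked door for the Habitacion_Victoria area that the player opens and closes with E when standing nearby.
; The Box overlap enables input, shows a prompt widget and opens a Gate; leaving reverses all three.
; E removes the prompt and, if the character has TieneLlave set, passes through the Gate to a FlipFlop.
; The FlipFlop alternately plays and reverses a Timeline that moves the Cube's relative location.
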(event OnComponentEndOverlap(Box)
  (params (OverlappedComponent :type Primitive%20Component%20Object%20Reference) (OtherActor :type Actor%20Object%20Reference) (OtherComp :type Primitive%20Component%20Object%20Reference) (OtherBodyIndex :type Integer))
  ;[1 1 1] colision personaje con puerta
  (Utilities|Casting|CastToBP_FirstPersonCharacter OtherActor)
  (Input|DisableInput (Game|GetPlayerController 0))
  ;[1 1 1] Aparece la indicacion y se va al apretar la "E" o alejarse de la puerta
  (Widget|RemovefromParent (stale OnComponentBeginOverlap(Box) _returnvalue))
  (Utilities|FlowControl|Gate true) ; enters at Close
)

(event OnComponentBeginOverlap(Box)
  (params (OverlappedComponent :type Primitive%20Component%20Object%20Reference) (OtherActor :type Actor%20Object%20Reference) (OtherComp :type Primitive%20Component%20Object%20Reference) (OtherBodyIndex :type Integer) (bFromSweep :type Boolean) (SweepResult :type Hit%20Result%20Structure%20%28by%20ref%29))
  ;[1 1 1] colision personaje con puerta
  (bind _asbp_first_person_character (Utilities|Casting|CastToBP_FirstPersonCharacter OtherActor))
  (Input|EnableInput (Game|GetPlayerController 0))
  ;[1 1 1] Aparece la indicacion y se va al apretar la "E" o alejarse de la puerta
  (bind _returnvalue (UserInterface|CreateWidget "/Game/Sample/Bluprints/InterfacePuerta.InterfacePuerta_C"))
  (UserInterface|Viewport|AddtoViewport _returnvalue 0)
  (Utilities|FlowControl|Gate true) ; enters at Open
)

(event Input|KeyboardEvents|E
  (params (Key :type Key%20Structure :default "None"))
  ;[1 1 1] Aparece la indicacion y se va al apretar la "E" o alejarse de la puerta
  (:Pressed
    (Widget|RemovefromParent (stale OnComponentBeginOverlap(Box) _returnvalue))
    ;[1 1 1] colision personaje con puerta
    (if (Variables|/Game/FirstPerson/Blueprints/BP_FirstPersonCharacter.BP_FirstPersonCharacter_C|GetTieneLlave? (stale OnComponentBeginOverlap(Box) _asbp_first_person_character))
      (Utilities|FlowControl|Gate true
        (:Exit
          ;[1 1 1] Abrir/cerrar puerta
          (Utilities|FlowControl|FlipFlop
            (:A
              (bind _puerta (Timeline|abirr/cerrar%20puerta Play)
                (:Update
                  (Transformation|SetRelativeLocation (Variables|Default|GetCube) _puerta false false))))
            (:B
              (Timeline|abirr/cerrar%20puerta Reverse))))))))

(fn ConstructionScript)