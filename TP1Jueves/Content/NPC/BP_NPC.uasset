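; BP_NPC is an NPC that wanders the level on its own.
; From BeginPlay, WalkNPC picks a random navigable point within a radius of the capsule's current location and uses AI MoveTo to walk there.
; It then calls itself again, after a pause on arrival or a much shorter delay on failure, forming an endless roaming loop.
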(event Custom|walkNPC
  (bind _randomlocation (Class|NavigationSystemV1|GetRandomLocationinNavigableRadius (Transformation|GetWorldLocation (Variables|Collision|GetCapsuleComponent)) (Variables|Default|GetRadius) (Variables|Default|GetNav%20Data) 0))
  (AI|AIMoveTo self _randomlocation 0 25.0 false
    (:OnSuccess
      (Utilities|FlowControl|Delay 3.0))
    (:OnFail
      (Utilities|FlowControl|Delay 0.1)))
  (CallFunction|WalkNPC))

(event EventBeginPlay
  (CallFunction|WalkNPC))

(fn ConstructionScript)